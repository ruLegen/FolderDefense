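; Procedural room Blueprint that lays out four walls from instances of a configurable wall mesh in its construction script.
; Each side places XCount instances, spaced by the mesh's bounds width along an axis rotated 90 degrees further per side.
; Each side starts one segment past the previous side's last instance, chaining the walls into a square loop.
; The event graph has no logic.
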(fn `UserConstructionScript`
  (locals (WallSize :type "Vector Structure"))
  (bind (_wallsize_x _wallsize_y) (`KismetMathLibrary.BreakVector` (`local.WallSize`)))
  (bind _wallinstancegroup (`self.WallInstanceGroup`))
  (bind (_wallsize_x_2 _wallsize_y_2) (`KismetMathLibrary.BreakVector` (`local.WallSize`)))
  (bind (_returnvalue_origin _returnvalue_boxextent) (`KismetMathLibrary.BreakBoxSphereBounds` (`StaticMesh.GetBounds` (`self.WallMesh`))))
  (set `local.WallSize` _returnvalue_boxextent)
  (`StaticMeshComponent.SetStaticMesh` (`self.WallInstanceGroup`) (`self.WallMesh`))
  (set `self.Rotation` 0.0)
  (for _index (range 4)
    (for _index_2 (range (`self.XCount`))
      (`InstancedStaticMeshComponent.AddInstance` (`self.WallInstanceGroup`) (`KismetMathLibrary.MakeTransform` (+ (`self.LastLocation`) (`KismetMathLibrary.RotateAngleAxis` (`KismetMathLibrary.MakeVector` 0.0 (* _index_2 (* 2 _wallsize_y))) (`self.Rotation`) (0.0 0.0 1.0))) (`KismetMathLibrary.MakeRotator` 0.0 0.0 (`self.Rotation`)))))
    (set `self.LastLocation` (+ (.location (`InstancedStaticMeshComponent.GetInstanceTransform` _wallinstancegroup (- (`InstancedStaticMeshComponent.GetInstanceCount` _wallinstancegroup) 1) false)) (`KismetMathLibrary.RotateAngleAxis` (`KismetMathLibrary.MakeVector` 0.0 (* 2 _wallsize_y_2)) (`self.Rotation`) (0.0 0.0 1.0))))
    (set `self.Rotation` (`KismetMathLibrary.Conv_IntToDouble` (* (+ _index 1) 90)))))